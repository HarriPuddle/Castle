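; BP_Enemy is a melee AI enemy that chases the player, deals damage on contact and respawns after death.
; Pawn sensing caches the spotted player, and Tick repeatedly issues AI MoveTo, applying damage while overlapping through a DoOnce reset by a one-second delay.
; Tick also updates a widget health bar and checks health directly.
; At zero health the enemy stops, then after a delay teleports to its respawn transform with full health.
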(event `self.ReceiveBeginPlay`
  (set `CharacterMovementComponent.MaxWalkSpeed` (`self.AI Speed`) (`self.CharacterMovement`))
  (set `self.EnemyHealth` (`self.EnemyBaseHealth`))
  (set `self.Dead` false))

(event `self.ReceiveTick`
  (params (DeltaSeconds :type "Float (single-precision)"))
  (`|ExecutionSequence`
    (:`then_0`
      (if (<= (`self.EnemyHealth`) 0.0)
        (set `self.Dead` true)
        (set `self.HasSeen` false)
        (`MovementComponent.StopMovementImmediately` (`self.CharacterMovement`))
        (elif (`self.HasSeen`)
          (`|AIMoveTo` self (0.0 0.0 0.0) (stale `self.PawnSensing.OnSeePawn` _asfirst_person_character)
            (:`then`
              (if (`self.IsOverlap`)
                (`/Engine/EditorBlueprintResources/StandardMacros.DoOnce` false :!label _label
                  (:`Completed`
                    (set `/Game/Broken/Blueprints/FirstPersonCharacter.Health` (- (`/Game/Broken/Blueprints/FirstPersonCharacter.Health` (stale `self.PawnSensing.OnSeePawn` _asfirst_person_character)) (`self.AI-Damage`)) (stale `self.PawnSensing.OnSeePawn` _asfirst_person_character))
                    (`KismetSystemLibrary.Delay` 1.0)
                    (goto _label :!via `Reset`)))))
            (:`OnSuccess`
              (set `self.IsOverlap` true))))))
    (:`then_1`
      (bind _ashealth_bar (cast `/Game/Broken/Blueprints/HealthBar` (`WidgetComponent.GetUserWidgetObject` (`self.Widget`))))
      (`ProgressBar.SetPercent` (`/Game/Broken/Blueprints/HealthBar.ProgressBar_60` _ashealth_bar) (/ (`self.EnemyHealth`) (`self.EnemyBaseHealth`))))
    (:`then_2`
      (if (`self.Dead`)
        (`KismetSystemLibrary.Delay` 2.5)
        (`self.K2_TeleportTo` (`self.RespawnLocationE`) (`self.RespawnRotationE`))
        (set `self.Dead` false)
        (set `self.EnemyHealth` (`self.EnemyBaseHealth`))))))

(event `self.PawnSensing.OnSeePawn`
  (params (Pawn :type "Pawn Object Reference"))
  (bind _asfirst_person_character (cast `/Game/Broken/Blueprints/FirstPersonCharacter` Pawn))
  (set `self.HasSeen` true))

(event `self.ReceiveActorBeginOverlap`
  (params (OtherActor :type "Actor Object Reference"))
  (cast `/Game/Broken/Blueprints/FirstPersonCharacter` OtherActor)
  (set `self.IsOverlap` true))

(event `self.ReceiveActorEndOverlap`
  (params (OtherActor :type "Actor Object Reference"))
  (cast `/Game/Broken/Blueprints/FirstPersonCharacter` OtherActor)
  (set `self.IsOverlap` false))

(fn `UserConstructionScript`)